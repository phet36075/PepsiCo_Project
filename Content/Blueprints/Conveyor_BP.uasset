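; Conveyor belt actor that carries any actor overlapping its Box along the forward direction of its StaticMesh.
; Each tick it offsets those actors by Speed scaled by delta time, without sweeping.
; The construction script puts a dynamic instance of Conveyor_M on the mesh, setting colour, arrow scale and scroll speed.
; The visual TrackSpeed is set independently of the movement Speed.
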(event `self.ReceiveTick`
  (params (DeltaSeconds :type "Float (single-precision)"))
  (for _array_element (`PrimitiveComponent.GetOverlappingActors` (`self.Box`) null)
    (`self.K2_AddActorWorldOffset` _array_element (* (`KismetMathLibrary.GetForwardVector` (`SceneComponent.K2_GetComponentRotation` (`self.StaticMesh`))) (* DeltaSeconds (`self.Speed`))) false false)))

(fn `UserConstructionScript`
  (bind _staticmesh (`self.StaticMesh`))
  (bind _returnvalue (`PrimitiveComponent.CreateDynamicMaterialInstance` _staticmesh 0 "/Game/Blueprints/Conveyor_M.Conveyor_M" "None"))
  (`PrimitiveComponent.SetMaterial` _staticmesh 0 _returnvalue)
  (`MaterialInstanceDynamic.SetVectorParameterValue` _returnvalue "Colour" (`self.Colour`))
  (`MaterialInstanceDynamic.SetScalarParameterValue` _returnvalue "X Scale" (`self.Arrow Scale`))
  (`MaterialInstanceDynamic.SetScalarParameterValue` _returnvalue "X Speed" (`self.Track Speed`)))