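; Spawner actor that emits a burst of Obj actors at its root component's world transform when play begins.
; A self-calling Loop event spawns one actor, increments CurrentIndex, then waits on a short Delay before repeating.
; The inclusive check against Amount runs after each spawn, so it produces Amount + 1 actors for non-negative values.
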(event `self.ReceiveBeginPlay`
  (set `self.CurrentIndex` 0)
  (`self.loop`))

(event `loop`
  (`|SpawnActorFromClass` (`self.Obj`) (`SceneComponent.K2_GetComponentToWorld` (`self.DefaultSceneRoot`)) "Undefined" "MultiplyWithRoot" null null)
  (set `self.CurrentIndex` (+ (`self.CurrentIndex`) 1))
  (`KismetSystemLibrary.Delay` 0.2)
  (if (<= (`self.CurrentIndex`) (`self.Amount`))
    (`self.loop`)))

(event `self.ReceiveTick`
  (params (DeltaSeconds :type "Float (single-precision)")))

(fn `UserConstructionScript`)